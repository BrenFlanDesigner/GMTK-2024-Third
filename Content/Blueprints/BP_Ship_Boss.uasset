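; Boss ship Blueprint that rams the player with a shielded boost and swings its projectile arrow.
; When the player enters its hazard collision, it thrusts, boosts and raises shields, then ends thrust and boost after a short delay.
; Shield sphere overlaps send the player damage based on ship size while boosting with shields up.
; A looping timer replays a timeline that rotates the arrow through an arc, varying its aim.
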(event `self.ReceiveBeginPlay`
  (`parent.ReceiveBeginPlay`)
  (`KismetSystemLibrary.K2_SetTimer` null "SwingShootArrow" 2.0 true))

(event `self.HazardCollision.OnComponentBeginOverlap`
  (params (OverlappedComponent :type "PrimitiveComponent Object Reference") (OtherActor :type "Actor Object Reference") (OtherComp :type "PrimitiveComponent Object Reference") (OtherBodyIndex :type Integer) (bFromSweep :type Boolean) (SweepResult :type "HitResult Structure (by ref)"))
  (if (`self.ActorHasTag` OtherActor "Player")
    (`self.ThrustStart`)
    (`self.Boost`)
    (`self.ActivateShields`)
    (`KismetSystemLibrary.Delay` 0.8)
    (`self.ThrustEnd`)
    (`self.StopBoosting`)))

(event `SwingShootArrow`
  (bind (_direction _newtrack_0) (`Timeline|TL_ProjectileArrowVariance]` :!via `PlayFromStart`)
    (:`Update`
      (`SceneComponent.K2_SetRelativeRotation` (`self.ShipArrow`) (`KismetMathLibrary.RLerp` (struct :`Yaw` 60.0) (struct :`Yaw` 120.0) _newtrack_0) false false))))

(event `self.ShieldSphere.OnComponentBeginOverlap`
  (params (OverlappedComponent :type "PrimitiveComponent Object Reference") (OtherActor :type "Actor Object Reference") (OtherComp :type "PrimitiveComponent Object Reference") (OtherBodyIndex :type Integer) (bFromSweep :type Boolean) (SweepResult :type "HitResult Structure (by ref)"))
  (`/Engine/EditorBlueprintResources/StandardMacros.IsValid` OtherActor
    (:`Is Valid`
      (if (and (`self.ActorHasTag` OtherActor "Player") (`self.IsBoosting?`) (`self.bAreShieldsUp`))
        (message `/Game/Blueprints/BPI_Combat.ConveyDamage` OtherActor (`self.ShipSize`))))))

(fn `UserConstructionScript`
  (`parent.UserConstructionScript`))