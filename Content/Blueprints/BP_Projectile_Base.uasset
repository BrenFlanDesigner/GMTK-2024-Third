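; Base projectile fired by a ship, which damages what it overlaps and destroys itself after a maximum number of hits.
; On BeginPlay it caches its owning BP_ShipParent and scales the HitBox by that ship's size.
; Overlaps ignore actors of the owner's or projectile's exact class; others receive ConveyDamageMessage carrying the owner's ShipSize.
; The construction script applies Speed to the projectile movement's initial and maximum speed.
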(event `self.ReceiveBeginPlay`
  (bind _asbp_ship_parent (cast `/Game/Blueprints/BP_ShipParent` (`self.GetOwner`)))
  (bind _output_get (set `self.OwningShip` _asbp_ship_parent))
  (bind _returnvalue (+ (* (`KismetMathLibrary.Conv_IntToDouble` (`/Game/Blueprints/BP_ShipParent.ShipSize` _output_get)) (`self.ScalePerShipSizeInteger`)) (`self.BaseProjectileScale`)))
  (`SceneComponent.SetWorldScale3D` (`self.HitBox`) (`KismetMathLibrary.MakeVector` _returnvalue _returnvalue _returnvalue)))

(event `self.HitBox.OnComponentBeginOverlap`
  (params (OverlappedComponent :type "PrimitiveComponent Object Reference") (OtherActor :type "Actor Object Reference") (OtherComp :type "PrimitiveComponent Object Reference") (OtherBodyIndex :type Integer) (bFromSweep :type Boolean) (SweepResult :type "HitResult Structure (by ref)"))
  (bind _returnvalue (`GameplayStatics.GetObjectClass` OtherActor))
  (if (and (!= _returnvalue (`GameplayStatics.GetObjectClass` (`self.OwningShip`))) (!= _returnvalue (`GameplayStatics.GetObjectClass` self)))
    (message `/Game/Blueprints/BPI_Combat.ConveyDamage` OtherActor (`/Game/Blueprints/BP_ShipParent.ShipSize` (`self.OwningShip`)))
    (bind _result (`/Engine/EditorBlueprintResources/StandardMacros.IncrementInt` (`self.NumberOfHits`))
      (:`  `
        (if (>= _result (`self.MaxHits`))
          (`self.K2_DestroyActor`))))))

(fn `UserConstructionScript`
  (bind _projectilemovement (`self.ProjectileMovement`))
  (bind _speed (`self.Speed`))
  (set `ProjectileMovementComponent.MaxSpeed` _speed _projectilemovement)
  (set `ProjectileMovementComponent.InitialSpeed` _speed _projectilemovement))