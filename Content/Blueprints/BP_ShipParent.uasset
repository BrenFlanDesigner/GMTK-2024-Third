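; Base ship class providing flight controls, projectile fire, shields, boost and health for derived ships.
; Timelines drive thrust, reverse and turning through movement input and player 0's control rotation, while timers manage boost fuel and shield regeneration.
; ShipSize sets scale and damage ratios, shields briefly block damage, and shielded boosting rams enemies.
; Empty hook functions signal scale, fuel and shield changes, and health updates feed a bar widget.
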(event `ThrustStart`
  ;[1 1 1] Basic Ship Controls
  ;;[1 0 0.01123] Thrust. Apply constant thrust when active, stop when stopped
  (`|ExecutionSequence`
    (:`then_0`
      (`Timeline|Timeline_1` :!label _label
        (:`Update`
          (`self.AddMovementInput` (`SceneComponent.GetForwardVector` (`self.ShipArrow`))))))
    (:`then_1`
      (bind _returnvalue (`GameplayStatics.SpawnSoundAttached` "/Game/Sounds/SFX_Thrust.SFX_Thrust" (`self.ShipArrow`) "None" (0.0 0.0 0.0) (struct) "KeepRelativeOffset" false 0.5 (`KismetMathLibrary.RandomFloatInRange` 0.9 1.1) 0.0 "/Game/Sounds/Attentuation_Standard.Attentuation_Standard" null))
      (set `self.ThrustSound` _returnvalue)
      (`self.TurnOnOffExhaust` true))))

(event `ThrustEnd`
  (bind _thrustsound (`self.ThrustSound`))
  ;[1 1 1] Basic Ship Controls
  ;;[1 0 0.01123] Thrust. Apply constant thrust when active, stop when stopped
  (`|ExecutionSequence`
    (:`then_0`
      (goto _label :!via `Stop`))
    (:`then_1`
      (`/Engine/EditorBlueprintResources/StandardMacros.IsValid` _thrustsound
        (:`Is Valid`
          (`AudioComponent.Stop` _thrustsound)
          (`GameplayStatics.PlaySoundAtLocation` "/Game/Sounds/SFX_Thrust_End.SFX_Thrust_End" (`self.K2_GetActorLocation`) (struct) 0.8 (`KismetMathLibrary.RandomFloatInRange` 0.9 1.1) 0.0 "/Game/Sounds/Attentuation_Standard.Attentuation_Standard" null null null)
          (`self.TurnOnOffExhaust` false))))))

(event `ReverseStart`
  ;[1 1 1] Basic Ship Controls
  ;;[0 0.3398 1] Reverse
  (`Timeline|Timeline_0` :!label _label_2
    (:`Update`
      (`self.AddMovementInput` (`SceneComponent.GetForwardVector` (`self.ShipArrow`)) -0.5))))

(event `ReverseEnd`
  ;[1 1 1] Basic Ship Controls
  ;;[0 0.3398 1] Reverse
  (goto _label_2 :!via `Stop`))

(event `TurnStart`
  (params (`Left?` :type Boolean))
  (bind (_returnvalue_roll _returnvalue_pitch _returnvalue_yaw) (`KismetMathLibrary.BreakRotator` (`self.GetControlRotation`)))
  ;[1 1 1] Basic Ship Controls
  ;;[0 1 0.2649] Turning
  (`Timeline|Timeline` :!label _label_3
    (:`Update`
      (`Controller.SetControlRotation` (`GameplayStatics.GetPlayerController` 0) (`KismetMathLibrary.MakeRotator` _returnvalue_roll _returnvalue_pitch (+ _returnvalue_yaw (* (`KismetMathLibrary.SelectFloat` -1.0 1.0 `Left?`) (`self.CurrentTurnSpeed`))))))))

(event `TurnEnd`
  ;[1 1 1] Basic Ship Controls
  ;;[0 1 0.2649] Turning
  (goto _label_3 :!via `Stop`))

(event `FireProjectile`
  (bind _shiparrow (`self.ShipArrow`))
  (bind _returnvalue (`SceneComponent.K2_GetComponentLocation` _shiparrow))
  (bind _returnvalue_2 (`SceneComponent.K2_GetComponentRotation` _shiparrow))
  ;[1 1 1] Basic Ship Controls
  ;;[0.5403 0 1] Fire Projectile
  (`|SpawnActorFromClass` (`self.ProjectileClass`) (`KismetMathLibrary.MakeTransform` _returnvalue _returnvalue_2) "Undefined" "MultiplyWithRoot" self self)
  (`GameplayStatics.PlaySoundAtLocation` "/Game/Sounds/laser_fire.laser_fire" _returnvalue (struct) 0.5 (`KismetMathLibrary.RandomFloatInRange` 0.9 1.1) 0.0 "/Game/Sounds/Attentuation_Standard.Attentuation_Standard" null null null)
  (`NiagaraFunctionLibrary.SpawnSystemAtLocation` "/Game/sA_Megapack_v1/sA_ShootingVfxPack/FX/NiagaraSystems/NS_AR_Muzzleflash_1_ONCE.NS_AR_Muzzleflash_1_ONCE" _returnvalue _returnvalue_2 (10.0 10.0 10.0)))

(event `ShowDamageNumber`
  (params (Value :type "Float (double-precision)"))
  (bind _damagenumber (`self.DamageNumber`))
  ;[0.9768 1 0] Flytext
  (`TextRenderComponent.K2_SetText` _damagenumber (`KismetTextLibrary.Conv_DoubleToText` Value "HalfToEven"))
  (`SceneComponent.SetHiddenInGame` _damagenumber false false)
  (`KismetSystemLibrary.Delay` 0.4)
  (`SceneComponent.SetHiddenInGame` (`self.DamageNumber`) true false))

(event `ScaleShip`
  (bind _returnvalue (+ (* (`KismetMathLibrary.Conv_IntToDouble` (`self.ShipSize`)) (`self.ScalePerShipSize`)) (`self.BaseShipScale`)))
  ;[0.7489 1 0.5909] HelperEvents
  (`SceneComponent.SetWorldScale3D` (`self.CapsuleComponent`) (`KismetMathLibrary.MakeVector` _returnvalue _returnvalue _returnvalue))
  (`self.OnShipScale`))

(event `SetMaxHealth`
  ;[0.7489 1 0.5909] HelperEvents
  (`/Game/Blueprints/AC_Health.InitializeMaxHealth` (`self.AC_Health`)))

(event `UpdateHP`
  (params (NewHP :type "Float (double-precision)"))
  ;[0.7489 1 0.5909] HelperEvents
  (message `/Game/Blueprints/BPI_EnemyShipFunctions.UpdateHealthBar` (`WidgetComponent.GetWidget` (`self.HealthBar`)) (/ NewHP (`/Game/Blueprints/AC_Health.MaxHealth` (`self.AC_Health`)))))

(event `self.ReceiveBeginPlay`
  ;[1 0 0.06297] BeginPlay
  (`self.UpdateHP` (`/Game/Blueprints/AC_Health.MaxHealth` (`self.AC_Health`)))
  (`self.ScaleShip`)
  (`KismetSystemLibrary.K2_SetTimer` null "BaseShieldReplenish" 2.5 true))

(event `SetShipSize`
  (params (NewShipSize :type Integer))
  ;[0.7489 1 0.5909] HelperEvents
  (set `self.ShipSize` NewShipSize)
  (`self.ScaleShip`))

(event `ActivateShields`
  (bind _shieldsphere (`self.ShieldSphere`))
  (bind _currentshieldvalue (`self.CurrentShieldValue`))
  (bind _shieldusecost (`self.ShieldUseCost`))
  ;[0.2587 0.2587 0.2587] Shields
  (if (>= _currentshieldvalue _shieldusecost)
    (set `self.CurrentShieldValue` (- _currentshieldvalue _shieldusecost))
    (`self.OnShieldConsume`)
    (`SceneComponent.SetHiddenInGame` _shieldsphere false false)
    (set `self.bAreShieldsUp` true)
    (`KismetSystemLibrary.Delay` 0.8)
    (`SceneComponent.SetHiddenInGame` _shieldsphere true false)
    (set `self.bAreShieldsUp` false)))

(event `Boost`
  (bind _charactermovement (`self.CharacterMovement`))
  ;[0.5229 0.003327 0.5938] Boost
  (if (>= (`self.CurrentBoostFuel`) (`self.MinimumFuelRequired`))
    (set `self.IsBoosting?` true)
    (set `CharacterMovementComponent.MaxAcceleration` (`self.BoostAcceleration`) _charactermovement)
    (set `CharacterMovementComponent.MaxFlySpeed` (`self.BoostFlySpeed`) _charactermovement)
    (set `self.CurrentTurnSpeed` (`self.BoostingTurnSpeed`))
    (`GameplayStatics.PlaySoundAtLocation` "/Game/Sounds/SFX_Boost.SFX_Boost" (`SceneComponent.K2_GetComponentLocation` (`self.ShipArrow`)) (struct) 1.0 (`KismetMathLibrary.RandomFloatInRange` 0.9 1.1) 0.0 "/Game/Sounds/Attentuation_Standard.Attentuation_Standard" null null null)
    (bind _returnvalue (`KismetSystemLibrary.K2_SetTimer` null "DecrimentFuel" 0.1 true))
    (set `self.DecrementFuelTImer` _returnvalue)))

(event `BaseShieldReplenish`
  (bind _maxshieldvalue (`self.MaxShieldValue`))
  (bind _returnvalue (+ (`self.CurrentShieldValue`) (`self.ShieldReplenishRate`)))
  ;[0.2587 0.2587 0.2587] Shields
  (if (>= _returnvalue _maxshieldvalue)
    (set `self.CurrentShieldValue` _maxshieldvalue)
    (else
      (set `self.CurrentShieldValue` _returnvalue)))
  (`self.OnShieldConsume`))

(event `StopBoosting`
  (bind _charactermovement (`self.CharacterMovement`))
  ;[0.5229 0.003327 0.5938] Boost
  (`|ExecutionSequence`
    (:`then_0`
      (set `self.IsBoosting?` false)
      (set `CharacterMovementComponent.MaxFlySpeed` (`self.DefaultFlySpeed`) _charactermovement)
      (set `CharacterMovementComponent.MaxAcceleration` (`self.DefaultAcceleration`) _charactermovement)
      (set `self.CurrentTurnSpeed` (`self.DefaultTurnSpeed`))
      (`KismetSystemLibrary.K2_ClearAndInvalidateTimerHandle` (`self.DecrementFuelTImer`)))
    (:`then_1`
      (`KismetSystemLibrary.Delay` 1.0)
      (`KismetSystemLibrary.K2_SetTimer` null "BaseFuelReplenish" 1.0 true false -0.5))))

(event `/Game/Blueprints/BPI_Combat.ConveyHeal`
  (params (HealAmount :type "Float (double-precision)"))
  ;[1 1 1] Heal Event
  (bind _newhealth (`/Game/Blueprints/AC_Health.AddHealth1` (`self.AC_Health`) HealAmount))
  (`self.UpdateHP` _newhealth))

(event `self.ShieldSphere.OnComponentBeginOverlap`
  (params (OverlappedComponent :type "PrimitiveComponent Object Reference") (OtherActor :type "Actor Object Reference") (OtherComp :type "PrimitiveComponent Object Reference") (OtherBodyIndex :type Integer) (bFromSweep :type Boolean) (SweepResult :type "HitResult Structure (by ref)"))
  ;[1 1 1] Ship Ramming While Boosting
  (`/Engine/EditorBlueprintResources/StandardMacros.IsValid` OtherActor
    (:`Is Valid`
      (if (and (`self.ActorHasTag` OtherActor "Enemy") (`self.IsBoosting?`) (`self.bAreShieldsUp`))
        (message `/Game/Blueprints/BPI_Combat.ConveyDamage` OtherActor (`self.ShipSize`))))))

(event `DecrimentFuel`
  (bind _returnvalue (- (`self.CurrentBoostFuel`) (`self.FuelConsumptionRate`)))
  ;[0.5229 0.003327 0.5938] Boost
  (if (<= _returnvalue 0.0)
    (set `self.CurrentBoostFuel` 0.0)
    (else
      (set `self.CurrentBoostFuel` _returnvalue)
      (`self.OnFuelConsume`))))

(event `BaseFuelReplenish`
  (bind _returnvalue (+ (`self.CurrentBoostFuel`) (`self.FuelConsumptionRate`)))
  ;[0.5229 0.003327 0.5938] Boost
  (if (>= _returnvalue (`self.MaxBoostFuel`))
    (set `self.CurrentBoostFuel` (`self.MaxBoostFuel`))
    (`self.OnFuelConsume`)
    (else
      (set `self.CurrentBoostFuel` _returnvalue)
      (`self.OnFuelConsume`))))

(fn `ConveyDamage`
  (params (InstigatorShipSize :type Integer))
  (returns (`bIsDead?` :type Boolean))
  (bind _returnvalue (* (/ (`KismetMathLibrary.Conv_IntToDouble` InstigatorShipSize) (`KismetMathLibrary.Conv_IntToDouble` (`self.ShipSize`))) (`self.BaseDamageValue`)))
  (if (not (`self.bAreShieldsUp`))
    (`self.ShowDamageNumber` (`KismetMathLibrary.Conv_IntToDouble` (`KismetMathLibrary.Round` _returnvalue)))
    (bind (_bisdead _newhp) (`/Game/Blueprints/AC_Health.TakeDamage1` (`self.AC_Health`) _returnvalue))
    (`self.UpdateHP` _newhp)
    (`|ExecutionSequence`
      (:`then_0`
        ;[1 1 1] Hit Sounds
        (`GameplayStatics.PlaySound2D` "/Game/Sounds/hitmarker.hitmarker" 0.25 (`KismetMathLibrary.RandomFloatInRange` 0.9 1.1) 0.0 null null)
        (`GameplayStatics.PlaySound2D` (select `int` (`KismetMathLibrary.RandomIntegerInRange` 0 2) :`0` "/Game/Sounds/bullet_impact_1.bullet_impact_1" :`1` "/Game/Sounds/bullet_impact_2.bullet_impact_2" :`2` "/Game/Sounds/bullet_impact_3.bullet_impact_3" :!type "SoundBase Object Reference") 0.7 (`KismetMathLibrary.RandomFloatInRange` 0.9 1.1) 0.0 null null))
      (:`then_1`
        (if _bisdead
          (`self.Die`))
        (return _bisdead)))))

(fn `Die`
  (bind _returnvalue (`self.K2_GetActorLocation`))
  (`NiagaraFunctionLibrary.SpawnSystemAtLocation` "/Game/sA_Megapack_v1/sA_ShootingVfxPack/FX/NiagaraSystems/NS_Explossion.NS_Explossion" _returnvalue (struct) (10.0 10.0 10.0))
  (`GameplayStatics.PlaySoundAtLocation` "/Game/Sounds/SFX_Explode.SFX_Explode" _returnvalue (struct) 1.0 (`KismetMathLibrary.RandomFloatInRange` 0.9 1.1) 0.0 "/Game/Sounds/Attentuation_Standard.Attentuation_Standard" null null null)
  (`PlayerController.ClientStartCameraShake` :`self` (`GameplayStatics.GetPlayerController` 0) :`Shake` "/Game/Blueprints/CS_Explosion.CS_Explosion_C"))

(fn `OnFuelConsume`)

(fn `OnShieldConsume`)

(fn `OnShipScale`)

(fn `TurnOnOffExhaust`
  (params (`Turn On` :type Boolean))
  (bind _exhaust2 (`self.Exhaust2`))
  (bind _exhaust3 (`self.Exhaust3`))
  (bind _exhaust4 (`self.Exhaust4`))
  (bind _exhaust1 (`self.Exhaust1`))
  (`|ExecutionSequence`
    (:`then_0`
      ;[1 1 1] Exhaust1
      (if (`self.Exhaust1Active?`)
        (if (`local.Turn On`)
          (`ActorComponent.Activate` _exhaust1 false)
          (else
            (`ActorComponent.Deactivate` _exhaust1)))))
    (:`then_1`
      ;[1 1 1] Exhaust2
      (if (`self.Exhaust2Active?`)
        (if (`local.Turn On`)
          (`ActorComponent.Activate` _exhaust2 false)
          (else
            (`ActorComponent.Deactivate` _exhaust2)))))
    (:`then_2`
      ;[1 1 1] Exhaust3
      (if (`self.Exhaust3Active?`)
        (if (`local.Turn On`)
          (`ActorComponent.Activate` _exhaust3 false)
          (else
            (`ActorComponent.Deactivate` _exhaust3)))))
    (:`then_3`
      ;[1 1 1] Exhaust1
      (if (`self.Exhaust4Active?`)
        (if (`local.Turn On`)
          (`ActorComponent.Activate` _exhaust4 false)
          (else
            (`ActorComponent.Deactivate` _exhaust4)))))))

(fn `UserConstructionScript`)