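; BP_BarkManager plays random 2D sound barks for spawn and defeat events.
; SendBark picks a clip from the matching array, keeping a reference to the spawn sound so a defeat bark can stop it before playing.
; A DoOnce reset by a five-second delay throttles all barks through one shared cooldown, so requests during that window are dropped, including defeat barks.
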(event `/Game/Blueprints/BPI_EnemyShipFunctions.SendBark`
  (params (Bark :type "/Game/Blueprints/E_BarkType Enum" :default "NewEnumerator0"))
  (bind _currentspawnbark (`self.CurrentSpawnBark`))
  (`/Engine/EditorBlueprintResources/StandardMacros.DoOnce` false :!label _label
    (:`Completed`
      (`|ExecutionSequence`
        (:`then_0`
          (switch `/Game/Blueprints/E_BarkType` Bark
            (:`NewEnumerator0`
              (bind _returnvalue (`GameplayStatics.CreateSound2D` (`KismetArrayLibrary.Array_Random` (`self.SpawnBarks`)) 1.0 1.0 0.0 null))
              (bind _output_get (set `self.CurrentSpawnBark` _returnvalue))
              (`AudioComponent.Play` _output_get 0.0))
            (:`NewEnumerator1`
              (`|ExecutionSequence`
                (:`then_0`
                  (`/Engine/EditorBlueprintResources/StandardMacros.IsValid` _currentspawnbark
                    (:`Is Valid`
                      (if (`AudioComponent.IsPlaying` _currentspawnbark)
                        (`AudioComponent.Stop` _currentspawnbark)))))
                (:`then_1`
                  (`GameplayStatics.PlaySound2D` (`KismetArrayLibrary.Array_Random` (`self.DefeatBarks`)) 1.0 1.0 0.0 null null))))))
        (:`then_1`
          (`KismetSystemLibrary.Delay` 5.0)
          (goto _label :!via `Reset`))))))

(fn `GetIsActive`
  (returns (bIsActive :type Boolean))
  (return false))

(fn `UserConstructionScript`)