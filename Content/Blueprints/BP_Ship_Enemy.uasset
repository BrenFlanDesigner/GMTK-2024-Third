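; Enemy ship Blueprint that is pooled and reused, starting hidden and parked out of the way.
; Spawn shows the mesh and resets health and its bar, while Thrust and Shoot wrap timed thrusting and projectile firing.
; On death it plays explosion effects, sound and camera shake, activates the first free pickup from a list cached at BeginPlay, then despawns itself for reuse.
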(event `self.ReceiveBeginPlay`
  (`self.Despawn`)
  (bind _outactors (`GameplayStatics.GetAllActorsOfClass` "/Game/Blueprints/BP_Base_Pickup.BP_Base_Pickup_C"))
  (set `self.PickupBPs` _outactors))

(event `Despawn`
  (`SceneComponent.SetHiddenInGame` (`self.ShipMesh`) true false)
  (set `self.Spawned` false)
  (`self.K2_SetActorLocation` (0.0 0.0 10000.0) false true))

(event `Spawn`
  (`SceneComponent.SetHiddenInGame` (`self.ShipMesh`) false false)
  (set `self.Spawned` true)
  (`self.SetMaxHealth`)
  (message `/Game/Blueprints/BPI_EnemyShipFunctions.UpdateHealthBar` (`WidgetComponent.GetWidget` (`self.HealthBar`)) 1.0))

(event `/Game/Blueprints/BPI_EnemyShipFunctions.Thrust`
  (params (ThrustDuration :type "Float (double-precision)"))
  (`self.ThrustStart`)
  (`KismetSystemLibrary.Delay` ThrustDuration)
  (`self.ThrustEnd`))

(event `/Game/Blueprints/BPI_EnemyShipFunctions.Shoot`
  (`self.FireProjectile`))

(fn `Die`
  (bind _returnvalue (`self.K2_GetActorLocation`))
  (`parent.Die`)
  (`|ExecutionSequence`
    (:`then_0`
      (`NiagaraFunctionLibrary.SpawnSystemAtLocation` "/Game/sA_Megapack_v1/sA_ShootingVfxPack/FX/NiagaraSystems/NS_Explossion.NS_Explossion" _returnvalue (struct) (10.0 10.0 10.0))
      (`GameplayStatics.PlaySoundAtLocation` "/Game/Sounds/SFX_Explode.SFX_Explode" _returnvalue (struct) 1.0 (`KismetMathLibrary.RandomFloatInRange` 0.9 1.1) 0.0 null null null null)
      (`PlayerController.ClientStartCameraShake` :`self` (`GameplayStatics.GetPlayerController` 0) :`Shake` "/Game/Blueprints/CS_Explosion.CS_Explosion_C" :`Scale` 0.5))
    (:`then_1`
      (for _array_element (`self.PickupBPs`)
        (if (not (`/Game/Blueprints/BP_Base_Pickup.bIsSpawned` _array_element))
          (`|ExecutionSequence`
            (:`then_0`
              (`/Game/Blueprints/BP_Base_Pickup.Spawn` _array_element (`self.K2_GetActorLocation`)))
            (:`then_1`
              (break))))))
    (:`then_2`
      (`self.Despawn`))))

(fn `UserConstructionScript`
  (`parent.UserConstructionScript`))