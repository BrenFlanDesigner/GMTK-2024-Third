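; BP_Pickup_FireRate is a pickup that makes the player ship fire faster by lowering its FireRate value.
; It overrides Pickup1 from its parent pickup class, calling the parent logic first.
; It then subtracts FireRateDecrease from the ship's FireRate, clamping the result so it never drops below MinimalFireRate.
; The event graph holds only disabled placeholder events.
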(fn `Pickup1`
  (params (PlayerShipBP :type "/Game/Blueprints/BP_Ship_Player Object Reference"))
  (bind _returnvalue (- (`/Game/Blueprints/BP_Ship_Player.FireRate` PlayerShipBP) (`self.FireRateDecrease`)))
  (`parent.Pickup1` PlayerShipBP)
  (if (<= _returnvalue (`self.MinimalFireRate`))
    (set `/Game/Blueprints/BP_Ship_Player.FireRate` (`self.MinimalFireRate`) PlayerShipBP)
    (else
      (set `/Game/Blueprints/BP_Ship_Player.FireRate` _returnvalue PlayerShipBP))))

(fn `UserConstructionScript`
  (`parent.UserConstructionScript`))