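; Enemy ship spawner that periodically activates ships from a pool of BP_Ship_Enemy actors gathered from the level at BeginPlay.
; A looping timer takes the first unspawned ship and picks a random XY point around the spawner.
; If a sphere trace sized to that ship finds the point clear, it teleports and spawns the ship.
; Ship size grows with the spawn-attempt counter and is reported to BP_GameManager.
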(event `self.ReceiveBeginPlay`
  (`KismetSystemLibrary.K2_SetTimer` null "SpawnShip" (`self.SpawnTimer`) true)
  (bind _outactors (`GameplayStatics.GetAllActorsOfClass` "/Game/Blueprints/BP_Ship_Enemy.BP_Ship_Enemy_C"))
  (set `self.EnemyObjectPool` _outactors)
  (bind _returnvalue (`GameplayStatics.GetActorOfClass` "/Game/Blueprints/BP_GameManager.BP_GameManager_C"))
  (bind _output_get (set `self.Manager` _returnvalue))
  (`KismetSystemLibrary.Delay` 0.2)
  (`/Game/Blueprints/BP_GameManager.UpdateEnemySize` _output_get (`self.ShipSizeToSpawn`)))

(event `SpawnShip`
  (bind _shiptospawn (`self.ShipToSpawn`))
  (for _array_element (`self.EnemyObjectPool`) :!label _label
    (if (not (`/Game/Blueprints/BP_Ship_Enemy.Spawned` _array_element))
      (`self.BreakLoop`)
      (bind _output_get (set `self.ShipToSpawn` _array_element))
      (`self.BreakLoop`)
      (bind _output_get_2 (set `self.SpawnLocation` (+ (`self.K2_GetActorLocation` self) (`KismetMathLibrary.MakeVector` (`KismetMathLibrary.RandomFloatInRange` -15000.0 15000.0) (`KismetMathLibrary.RandomFloatInRange` -15000.0 15000.0)))))
      (bind (_outhits _returnvalue) (`KismetSystemLibrary.SphereTraceMulti` _output_get_2 _output_get_2 (`KismetMathLibrary.Conv_IntToDouble` (* (`/Game/Blueprints/BP_ShipParent.ShipSize` _output_get) 20)) "TraceTypeQuery1"))
      (if (not _returnvalue)
        (`self.K2_SetActorLocation` _shiptospawn (`self.SpawnLocation`) false true)
        (bind _output_get_3 (set `self.ShipSizeToSpawn` (/ (`self.ShipsSpawned`) 3)))
        (`/Game/Blueprints/BP_ShipParent.SetShipSize` _shiptospawn _output_get_3)
        (`/Game/Blueprints/BP_Ship_Enemy.Spawn` _shiptospawn)
        (`/Game/Blueprints/BP_GameManager.UpdateEnemySize` (`self.Manager`) (`self.ShipSizeToSpawn`)))))
  (`/Engine/EditorBlueprintResources/StandardMacros.IncrementInt` (`self.ShipsSpawned`)))

(event `BreakLoop`
  (goto _label :!via `Break`))

(fn `UserConstructionScript`)