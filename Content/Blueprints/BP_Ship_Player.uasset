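; Player-controlled ship Blueprint, extending a parent ship with input, camera and UI feedback.
; Input drives thrust, turning, boost, shields, clamped zoom, pause, slow precise aiming and held fire via a looping timer behind a rate-limiting DoOnce.
; Parent overrides push size, fuel and shield values to BP_GameManager and ship widgets, and scale fly speed with ship size.
; Death disables and hides the ship, then shows the game-over screen after a delay.
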(event `InputAction|Thrust`
  (params (Key :type "Key Structure"))
  ;[1 1 1] Control Thrust
  (:`Pressed`
    (`self.ThrustStart`))
  (:`Released`
    (`self.ThrustEnd`)))

(event `self.ReceiveBeginPlay`
  (bind _charactermovement (`self.CharacterMovement`))
  ;[1 0.02922 0] BeginPlay
  (`parent.ReceiveBeginPlay`)
  (bind _returnvalue (`GameplayStatics.GetActorOfClass` "/Game/Blueprints/BP_GameManager.BP_GameManager_C"))
  (set `self.Manager` _returnvalue)
  (`self.UpdateShipSizeUI`)
  (`self.OnShieldConsume`)
  (`self.OnFuelConsume`)
  (set `CharacterMovementComponent.MaxFlySpeed` (`self.DefaultFlySpeed`) _charactermovement)
  (set `CharacterMovementComponent.MaxAcceleration` (`self.DefaultAcceleration`) _charactermovement))

(event `InputAction|Reverse`
  (params (Key :type "Key Structure"))
  ;[1 1 1] Control Reverse
  (:`Pressed`
    (`self.ReverseStart`))
  (:`Released`
    (`self.ReverseEnd`)))

(event `InputAxis|Turn`
  (params (AxisValue :type "Float (single-precision)"))
  ;[1 1 1] Turn Control
  (if (> AxisValue 0.1)
    (`self.TurnStart` true)
    (elif (< AxisValue -0.1)
      (`self.TurnStart` false)
      (else
        (`self.TurnEnd`)))))

(event `FireBcHolding`
  ;[1 0.7677 0] FirCode
  (`/Engine/EditorBlueprintResources/StandardMacros.DoOnce` false :!label _label
    (:`Completed`
      (bind _returnvalue (`KismetSystemLibrary.K2_SetTimer` null "FireSingleShot" (`self.FireRate`) true false (* (`self.FireRate`) -1.0)))
      (set `self.FiringTimer` _returnvalue)
      (`PlayerController.ClientStartCameraShake` :`self` (`GameplayStatics.GetPlayerController` 0) :`Shake` "/Game/Blueprints/CS_Recoil.CS_Recoil_C" :`Scale` 0.025)
      (`KismetSystemLibrary.Delay` (`self.FireRate`))
      (`self.ResetFireDoOnce`)
      (if (`self.bIsHoldingFire`)
        (`self.FireBcHolding`)))))

(event `InputAction|Shoot`
  (params (Key :type "Key Structure"))
  ;[1 0.7677 0] FirCode
  (:`Pressed`
    (set `self.bIsHoldingFire` true)
    (goto _label))
  (:`Released`
    (set `self.bIsHoldingFire` false)
    (`KismetSystemLibrary.K2_ClearAndInvalidateTimerHandle` (`self.FiringTimer`))))

(event `ResetFireDoOnce`
  ;[1 0.7677 0] FirCode
  (goto _label :!via `Reset`))

(event `FireSingleShot`
  ;[1 0.7677 0] FirCode
  (`self.FireProjectile`))

(event `InputAction|PreciseAIm`
  (params (Key :type "Key Structure"))
  (bind _cylinder (`self.Cylinder`))
  ;[0 1 0.9227] SlowRotation for PreciseAiming
  (:`Pressed`
    (set `self.bIsAiming` true)
    (set `self.CurrentTurnSpeed` (`self.PreciseAimTurnSpeed`))
    (`SceneComponent.SetHiddenInGame` _cylinder false true)
    (set `SpringArmComponent.TargetArmLength` (`SpringArmComponent.TargetArmLength` (`self.CameraSpringArm`)) (`self.CrossHairSpringArm`)))
  (:`Released`
    (set `self.bIsAiming` false)
    (set `self.CurrentTurnSpeed` (`self.DefaultTurnSpeed`))
    (`SceneComponent.SetHiddenInGame` _cylinder true true)))

(event `InputAction|Boost`
  (params (Key :type "Key Structure"))
  ;[1 1 1] Fuel/Boost Stuff
  (:`Pressed`
    (`self.Boost`)
    (`PlayerController.ClientStartCameraShake` :`self` (`GameplayStatics.GetPlayerController` 0) :`Shake` "/Game/Blueprints/CS_Boost.CS_Boost_C" :`Scale` 0.1))
  (:`Released`
    (`self.StopBoosting`)
    (set `self.LetGoOfBoosting` true)
    (set `self.CurrentTurnSpeed` (`self.PostBoostTurnSpeedBuffed`))
    (`KismetSystemLibrary.Delay` 0.3)
    (if (not (`self.bIsAiming`))
      (set `self.CurrentTurnSpeed` (`self.DefaultTurnSpeed`)))))

(event `InputAction|ZoomOut`
  (params (Key :type "Key Structure"))
  (bind _cameraspringarm (`self.CameraSpringArm`))
  (bind _returnvalue (+ (`SpringArmComponent.TargetArmLength` (`self.CameraSpringArm`)) (`self.ZoomIncrement`)))
  ;[0 1 0.4764] ZoomFeature
  (:`Pressed`
    (if (>= _returnvalue (`self.MaxSpringArmLength`))
      (set `SpringArmComponent.TargetArmLength` (`self.MaxSpringArmLength`) _cameraspringarm)
      (else
        (set `SpringArmComponent.TargetArmLength` _returnvalue _cameraspringarm)))))

(event `self.StopBoosting`
  ;[1 1 1] Fuel/Boost Stuff
  (`parent.StopBoosting`)
  (`PlayerController.ClientStopCameraShake` (`GameplayStatics.GetPlayerController` 0) "/Game/Blueprints/CS_Boost.CS_Boost_C" true))

(event `FuelPickupUpdate`
  ;[1 1 1] Fuel/Boost Stuff
  ;;[1 0 0.6484] Boost Fuel Update
  (`self.OnFuelConsume`))

(event `InputAction|ZoomIn`
  (params (Key :type "Key Structure"))
  (bind _cameraspringarm (`self.CameraSpringArm`))
  (bind _returnvalue (- (`SpringArmComponent.TargetArmLength` (`self.CameraSpringArm`)) (`self.ZoomIncrement`)))
  ;[0 1 0.4764] ZoomFeature
  (:`Pressed`
    (if (<= _returnvalue (`self.BaseSprimArmLength`))
      (set `SpringArmComponent.TargetArmLength` (`self.BaseSprimArmLength`) _cameraspringarm)
      (else
        (set `SpringArmComponent.TargetArmLength` _returnvalue _cameraspringarm)))))

(event `UpdateShipSizeUI`
  (`/Game/Blueprints/BP_GameManager.UpdatePlayerSize` (`self.Manager`) (`self.ShipSize`)))

(event `InputAction|ActivateShields`
  (params (Key :type "Key Structure"))
  ;[0 0.01424 1] Activate Shield
  (:`Pressed`
    (`self.ActivateShields`)
    (`PlayerController.ClientStartCameraShake` :`self` (`GameplayStatics.GetPlayerController` 0) :`Shake` "/Game/Blueprints/CS_Explosion.CS_Explosion_C" :`Scale` 0.05)
    (`GameplayStatics.PlaySoundAtLocation` "/Game/Sounds/SFX_Shield.SFX_Shield" (`self.K2_GetActorLocation`) (struct) 1.0 (`KismetMathLibrary.RandomFloatInRange` 0.9 1.1) 0.0 "/Game/Sounds/Attentuation_Standard.Attentuation_Standard" null null null)))

(event `DeathScreen`
  (bind _returnvalue (`GameplayStatics.GetPlayerController` 0))
  ;[0.3073 0 0] Game Over Screen
  (`/Engine/EditorBlueprintResources/StandardMacros.DoOnce` false
    (:`Completed`
      (`|ExecutionSequence`
        (:`then_0`
          (`|ExecutionSequence`
            (:`then_0`
              _)
            (:`then_1`
              _))
          (bind _returnvalue_2 (`GameplayStatics.GetActorOfClass` "/Script/Engine.AmbientSound"))
          (`/Engine/EditorBlueprintResources/StandardMacros.IsValid` _returnvalue_2
            (:`Is Valid`
              (`self.K2_DestroyActor` _returnvalue_2))))
        (:`then_1`
          (`self.DisableInput` _returnvalue)
          (`self.SetActorHiddenInGame` true)
          (set `PlayerController.bShowMouseCursor` true _returnvalue)
          (`self.SetActorEnableCollision` false))
        (:`then_2`
          (`KismetSystemLibrary.Delay` 2.0)
          (bind _returnvalue_3 (`|CreateWidget` "/Game/Blueprints/UI/WBP_GameOver.WBP_GameOver_C"))
          (`UserWidget.AddToViewport` _returnvalue_3 0))))))

(event `InputAction|Pause`
  (params (Key :type "Key Structure"))
  (:`Pressed`
    (bind _returnvalue (`|CreateWidget` "/Game/Blueprints/UI/WBP_PauseMenu.WBP_PauseMenu_C"))
    (bind _output_get (set `self.PauseMenu` _returnvalue))
    (`UserWidget.AddToViewport` _output_get 0)))

(fn `Die`
  (`parent.Die`)
  (`self.DeathScreen`))

(fn `GivePlayerShipBP`
  (returns (PlayerBP :type "/Game/Blueprints/BP_Ship_Player Object Reference"))
  (return self))

(fn `OnFuelConsume`
  (bind _returnvalue (/ (`self.CurrentBoostFuel`) (`self.MaxBoostFuel`)))
  (`parent.OnFuelConsume`)
  (`/Game/Blueprints/BP_GameManager.UpdateFuelBar` (`self.Manager`) _returnvalue)
  (message `/Game/Blueprints/BPI_Combat.UpdateFuelDisplay` (`WidgetComponent.GetWidget` (`self.Fuel`)) _returnvalue))

(fn `OnShieldConsume`
  (bind _returnvalue (/ (`self.CurrentShieldValue`) (`self.MaxShieldValue`)))
  (`parent.OnShieldConsume`)
  (message `/Game/Blueprints/BPI_Combat.UpdateFuelDisplay` (`WidgetComponent.GetWidget` (`self.Shieldvalue`)) _returnvalue)
  (`/Game/Blueprints/BP_GameManager.UpdateShieldBar` (`self.Manager`) _returnvalue))

(fn `OnShipScale`
  (bind _charactermovement (`self.CharacterMovement`))
  (`parent.OnShipScale`)
  (set `CharacterMovementComponent.MaxFlySpeed` (+ (`CharacterMovementComponent.MaxFlySpeed` _charactermovement) (* (`self.ShipSize`) (`self.MoveSpeedPerSizeInt`))) _charactermovement))

(fn `UserConstructionScript`
  (`parent.UserConstructionScript`))