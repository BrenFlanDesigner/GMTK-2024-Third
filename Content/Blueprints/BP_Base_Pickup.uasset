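; Base pickup actor that the player collects by touching it, built to be reused rather than destroyed.
; It starts despawned, hidden and moved far below the world, until Spawn shows it at a given location.
; When a Player-tagged actor overlaps its volume, it fetches the player ship through a message call and runs Pickup1.
; Pickup1 plays a pitch-randomized sound and despawns it, leaving the passed ship unused.
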(event `self.ReceiveBeginPlay`
  (`self.DeSpawn`))

(event `DeSpawn`
  (`SceneComponent.SetHiddenInGame` (`self.PickupMesh`) true true)
  (`SceneComponent.K2_SetWorldLocation` (`self.DefaultSceneRoot`) (0.0 0.0 -10000.0) false true)
  (set `self.bIsSpawned` false))

(event `Spawn`
  (params (SpawnLoc :type "Vector Structure"))
  (`SceneComponent.SetHiddenInGame` (`self.PickupMesh`) false true)
  (`SceneComponent.K2_SetWorldLocation` (`self.DefaultSceneRoot`) SpawnLoc false true)
  (set `self.bIsSpawned` true))

(event `self.OverlapVolume.OnComponentBeginOverlap`
  (params (OverlappedComponent :type "PrimitiveComponent Object Reference") (OtherActor :type "Actor Object Reference") (OtherComp :type "PrimitiveComponent Object Reference") (OtherBodyIndex :type Integer) (bFromSweep :type Boolean) (SweepResult :type "HitResult Structure (by ref)"))
  (if (`self.ActorHasTag` OtherActor "Player")
    (bind _playerbp (message `/Game/Blueprints/BPI_Pickups.GivePlayerShipBP` OtherActor))
    (`self.Pickup1` _playerbp)))

(fn `Pickup1`
  (params (PlayerShipBP :type "/Game/Blueprints/BP_Ship_Player Object Reference"))
  (`GameplayStatics.PlaySoundAtLocation` (`self.PickupSFX`) (`self.K2_GetActorLocation`) (struct) 1.0 (`KismetMathLibrary.RandomFloatInRange` 0.9 1.1) 0.0 null null null null)
  (`self.DeSpawn`))

(fn `UserConstructionScript`)