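; AC_Health is a health component that tracks current health, maximum health and death state, intended for BP_ShipParent actors.
; BeginPlay caches the owner as a BP_ShipParent, while a separate InitializeMaxHealth event fills current health to the maximum.
; TakeDamage1 clamps health at zero, sets IsDead and returns both values.
; AddHealth1 caps healing at the maximum and returns the new health, leaving IsDead untouched.
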(event `InitializeMaxHealth`
  (set `self.CurrentHealth` (`self.MaxHealth`)))

(event `self.ReceiveBeginPlay`
  (bind _asbp_ship_parent (cast `/Game/Blueprints/BP_ShipParent` (`self.GetOwner`)))
  (set `self.OwningActor` _asbp_ship_parent))

(fn `AddHealth1`
  (params (HealValue :type "Float (double-precision)"))
  (returns (NewHealth :type "Float (double-precision)"))
  (bind _returnvalue (+ HealValue (`self.CurrentHealth`)))
  (if (>= _returnvalue (`self.MaxHealth`))
    (bind _output_get (set `self.CurrentHealth` (`self.MaxHealth`)))
    (return _output_get)
    (else
      (bind _output_get_2 (set `self.CurrentHealth` _returnvalue))
      (return _output_get_2))))

(fn `TakeDamage1`
  (params (DamageValue :type "Float (double-precision)"))
  (returns (bIsDead :type Boolean) (NewHP :type "Float (double-precision)"))
  (bind _returnvalue (- (`self.CurrentHealth`) DamageValue))
  (if (<= _returnvalue 0.0)
    (set `self.bIsDead` true)
    (bind _output_get (set `self.CurrentHealth` 0.0))
    (return true _output_get)
    (else
      (bind _output_get_2 (set `self.CurrentHealth` _returnvalue))
      (return false _output_get_2))))