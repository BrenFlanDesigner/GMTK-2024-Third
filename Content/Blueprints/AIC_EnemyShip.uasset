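; AI controller for enemy ships that attacks players it detects through AI Perception while the controlled ship is active.
; On sensing a Player-tagged actor, it focuses on it, halts random patrol, thrusts, and starts looping timers for firing and repeated thrust.
; Losing the player clears focus and both timers, then resumes patrol.
; All ship actions go through message calls on the pawn, leaving movement and shooting to the ship.
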(event `self.ReceiveBeginPlay`)

(event `self.AIPerception.OnTargetPerceptionUpdated`
  (params (Actor :type "Actor Object Reference") (Stimulus :type "AIStimulus Structure"))
  (bind _returnvalue (`self.K2_GetPawn`))
  (bind _bisactive (message `/Game/Blueprints/BPI_EnemyShipFunctions.GetIsActive` (`self.K2_GetPawn`)))
  (if _bisactive
    (if (`self.ActorHasTag` Actor "Player")
      (if (`.bSuccessfullySensed` (break `AIStimulus` Stimulus))
        (`self.K2_SetFocus` Actor)
        (message `/Game/Blueprints/BPI_EnemyShipFunctions.RandomPatrolOrder` _returnvalue false)
        (message `/Game/Blueprints/BPI_EnemyShipFunctions.Thrust` _returnvalue 0.75)
        (bind _returnvalue_2 (`KismetSystemLibrary.K2_SetTimer` null "Fire" (`self.FireRate`) true))
        (set `self.FireTimer` _returnvalue_2)
        (bind _returnvalue_3 (`KismetSystemLibrary.K2_SetTimer` null "ThrustAgain" 5.0 true))
        (set `self.ThrustTimer` _returnvalue_3)
        (else
          (`self.K2_ClearFocus`)
          (`KismetSystemLibrary.K2_ClearAndInvalidateTimerHandle` (`self.FireTimer`))
          (`KismetSystemLibrary.K2_ClearAndInvalidateTimerHandle` (`self.ThrustTimer`))
          (message `/Game/Blueprints/BPI_EnemyShipFunctions.RandomPatrolOrder` (`self.K2_GetPawn`) true))))))

(event `Fire`
  (message `/Game/Blueprints/BPI_EnemyShipFunctions.Shoot` (`self.K2_GetPawn`)))

(event `ThrustAgain`
  (message `/Game/Blueprints/BPI_EnemyShipFunctions.Thrust` (`self.K2_GetPawn`) 0.75))

(fn `UserConstructionScript`)